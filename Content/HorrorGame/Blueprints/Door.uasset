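; Horror game door Blueprint that swings open and closed, with a sound for each, when its OpenClose event fires.
; A FlipFlop alternates calls: opening captures the current rotation plus a 90-degree yaw target and plays the SmoothDoorG timeline, which lerps the root component's rotation between them.
; Closing reverses the same timeline at a faster play rate, so the door opens slowly and shuts quickly.
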(event `OpenClose`
  (bind _smoothdoorg (`self.SmoothDoorG`))
  (bind _returnvalue (`SceneComponent.K2_GetComponentLocation` (`self.Door`)))
  (bind _returnvalue_2 (`SceneComponent.K2_GetComponentRotation` (`self.DefaultSceneRoot`)))
  (`/Engine/EditorBlueprintResources/StandardMacros.FlipFlop`
    (:`A`
      (set `self.Base Rotation` _returnvalue_2)
      (set `self.Target Rotation` (`KismetMathLibrary.MakeRotator` (.roll _returnvalue_2) (.pitch _returnvalue_2) (+ (.yaw _returnvalue_2) 90.0)))
      (`TimelineComponent.SetPlayRate` _smoothdoorg 0.3)
      (`GameplayStatics.PlaySoundAtLocation` "/Game/HorrorGame/Sounds/doorOpen.doorOpen" _returnvalue (struct) 1.0 1.0 0.0 null null null)
      (bind (_direction _doormovement) (`Timeline|SmoothDoorG` :!label _label)
        (:`Update`
          (`SceneComponent.K2_SetWorldRotation` (`self.DefaultSceneRoot`) (`KismetMathLibrary.RLerp` (`self.Base Rotation`) (`self.Target Rotation`) _doormovement) false false))))
    (:`B`
      (`TimelineComponent.SetPlayRate` _smoothdoorg 1.1)
      (`GameplayStatics.PlaySoundAtLocation` "/Game/HorrorGame/Sounds/doorClose.doorClose" _returnvalue (struct) 1.0 1.0 0.0 null null null)
      (goto _label :!via `Reverse`))))

(fn `UserConstructionScript`)